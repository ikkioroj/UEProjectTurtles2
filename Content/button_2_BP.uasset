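; A pushable button that spawns a Turtle1 actor at a fixed world location when the player interacts with it.
; Box overlap with the third-person character opens a gate, so the Interact input only works while the player is inside the box.
; A collapsed animation graph plays a click sound and uses a timeline to lerp the button mesh to a pressed-in position before the spawn.
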(event OnComponentBeginOverlap(Box)
  (params (OverlappedComponent :type Primitive%20Component%20Object%20Reference) (OtherActor :type Actor%20Object%20Reference) (OtherComp :type Primitive%20Component%20Object%20Reference) (OtherBodyIndex :type Integer) (bFromSweep :type Boolean) (SweepResult :type Hit%20Result%20Structure%20%28by%20ref%29))
  ;[1 1 1] button interaction (push button)
  (Utilities|Casting|CastToBP_ThirdPersonCharacter OtherActor)
  (Utilities|FlowControl|Gate true) ; enters at Open
)

(event OnComponentEndOverlap(Box)
  (params (OverlappedComponent :type Primitive%20Component%20Object%20Reference) (OtherActor :type Actor%20Object%20Reference) (OtherComp :type Primitive%20Component%20Object%20Reference) (OtherBodyIndex :type Integer))
  ;[1 1 1] button interaction (push button)
  (Utilities|Casting|CastToBP_ThirdPersonCharacter OtherActor)
  (Utilities|FlowControl|Gate true) ; enters at Close
)

(event EventBeginPlay
  (bind _button1 (Variables|Default|GetButton1))
  (bind _returnvalue (Transformation|GetRelativeTransform _button1))
  (Variables|Default|SetOutPos (Math|Transform|MakeTransform (.location _returnvalue) (.rotation _returnvalue) (.scale _returnvalue)))
  (Variables|Default|SetInPos (Math|Transform|MakeTransform (- (.location _returnvalue) "0.000000,10.000000,0.000000") (.rotation _returnvalue) (.scale _returnvalue)))
  (Input|EnableInput (Game|GetPlayerController 0)))

(event Input|ActionEvents|InputActionInteract
  (params (Key :type Key%20Structure :default "None"))
  ;[1 1 1] button interaction (push button)
  (:Pressed
    (Utilities|FlowControl|Gate true
      (:Exit
        ;[1 1 1] button moving animation
        (|buttonAnimation
          (:out
            (Game|SpawnActorfromClass "/Game/StarterContent/Blueprints/turtle1.turtle1_C" (Math|Transform|MakeTransform "1800.000000,1500.000000,100.000000" "0, 0, 0" "1.000000,1.000000,1.000000") "Undefined" 0 0)))))))

(fn ConstructionScript)